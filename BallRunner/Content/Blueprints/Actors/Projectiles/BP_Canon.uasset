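; BP_Canon is a cannon actor that automatically fires projectiles in an endless loop from BeginPlay.
; Each cycle waits FireRate seconds, then spawns a BP_Bullet at the Arrow component's world location and rotation, scaled by BulletScale.
; The CanonMovement timeline then animates the Cannon component's relative Y position.
; Its completion restarts the cycle, so the shot interval is the delay plus the animation length.
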(event EventBeginPlay
  (Utilities|FlowControl|Delay (Variables|CannonProperties|GetFireRate) :!label _label)
  (CallFunction|SpawnBullet)
  (bind _canony (Timeline|CanonMovement PlayFromStart)
    (:Update
      (CallFunction|CannonYAnimation _canony))
    (:Finished
      (goto _label))))

(event Collision|EventActorBeginOverlap
  (params (OtherActor :type Actor%20Object%20Reference)))

(event EventTick
  (params (DeltaSeconds :type Float%20%28single-precision%29)))

(fn ConstructionScript)

(fn SpawnBullet
  (bind _arrow (Variables|Default|GetArrow))
  (Game|SpawnActorfromClass "/Game/Blueprints/Actors/Projectiles/BP_Bullet.BP_Bullet_C" (Math|Transform|MakeTransform (Transformation|GetWorldLocation _arrow) (Transformation|GetWorldRotation _arrow) (Math|Conversions|ToVector(Float) (Variables|CannonProperties|GetBulletScale))) "Undefined" 0 0))

(fn CannonYAnimation
  (params (CannonY :type Float%20%28single-precision%29))
  (Transformation|SetRelativeLocation (Variables|Default|Getcannon) (Math|Vector|MakeVector 0.0 CannonY 0.0) false false))