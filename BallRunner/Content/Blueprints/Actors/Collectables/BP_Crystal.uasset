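; BP_Crystal is a collectable crystal that flies into the player and vanishes when the player overlaps it.
; On overlap it caches its location, scale and point light intensity, then plays the TL_BlendAlpha timeline.
; Separate timeline curves lerp it toward the player's live position, shrink it to zero and fade its light out.
; The actor destroys itself when the timeline finishes.
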(event EventBeginPlay)

(event Collision|EventActorBeginOverlap
  (params (OtherActor :type Actor%20Object%20Reference))
  (Utilities|IsPlayer OtherActor
    (:IsPlayer
      (CallFunction|ObjectProperties)
      (bind (_direction _smoothlerpalpha _objectscale _lightintensity) (Timeline|TL_BlendAlpha Play)
        (:Update
          (CallFunction|MoveObjecttoPlayer _smoothlerpalpha)
          (CallFunction|ScaleObject _objectscale)
          (CallFunction|ChangeLightIntensity _lightintensity))
        (:Finished
          (Actor|DestroyActor))))))

(event EventTick
  (params (DeltaSeconds :type Float%20%28single-precision%29)))

(fn ConstructionScript)

(fn MoveObjecttoPlayer
  (params (Alpha :type Float%20%28single-precision%29))
  (Transformation|SetActorLocation (Math|Vector|Lerp(Vector) (Variables|Default|GetCrystalLocation) (Transformation|GetActorLocation (Game|Player|GetPlayerPawn 0)) Alpha) false false))

(fn ObjectProperties
  (Variables|Default|SetCrystalLocation (Transformation|GetActorLocation))
  (Variables|Default|SetStartCrystalScale (Transformation|GetActorScale3D))
  (Variables|Default|SetLerpStartIntensity (Variables|/Script/Engine.LightComponentBase|GetIntensity (Variables|Default|GetPointLight))))

(fn ScaleObject
  (params (Alpha :type Float%20%28single-precision%29))
  (Transformation|SetActorScale3D (Math|Vector|Lerp(Vector) (Variables|Default|GetStartCrystalScale) "0, 0, 0" Alpha)))

(fn ChangeLightIntensity
  (params (Alpha :type Float%20%28single-precision%29))
  (Rendering|Components|Light|SetIntensity (Variables|Default|GetPointLight) (Math|Float|Lerp (Variables|Default|GetLerpStartIntensity) 0.0 Alpha)))